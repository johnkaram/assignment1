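; Button Blueprint that, once pressed, starts continuously spawning bombs inside a box area.
; ButtonPressed runs the parent logic, then starts a looping two-second timer stored in Timer, which this Blueprint never clears.
; Each tick of that timer fires SpawnBOMB, placing a BP_BOMB at a random point within Box1's bounds, using the scaled extent rotated by the box's world rotation.
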(event `self.button_pressed`
  (`parent.button_pressed`)
  (bind _returnvalue (`KismetSystemLibrary.K2_SetTimerDelegate` (delegate `Spawn BOMB`) 2.0 true))
  (set `self.timer` _returnvalue))

(event `Spawn BOMB`
  (bind _box1 (`self.Box1`))
  (`|SpawnActorFromClass` "/Game/BP_BOMB.BP_BOMB_C" (`KismetMathLibrary.MakeTransform` (`KismetMathLibrary.RandomPointInBoundingBox` (`SceneComponent.K2_GetComponentLocation` _box1) (`KismetMathLibrary.GreaterGreater_VectorRotator` (`BoxComponent.GetScaledBoxExtent` _box1) (`SceneComponent.K2_GetComponentRotation` _box1)))) "Undefined" "OverrideRootScale" null null))

(fn `UserConstructionScript`
  (`parent.UserConstructionScript`))