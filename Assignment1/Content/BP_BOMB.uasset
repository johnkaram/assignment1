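; BP_BOMB is a bomb that knocks nearby UFOs out of their animation and blasts them away with physics when it hits something.
; On Hit, it runs a sphere overlap for WorldDynamic objects around itself and casts the found actors to BP-UFO.
; Each UFO gets physics simulation enabled on its mesh, its UFOAnimation stopped, and a constant-falloff radial impulse applied from the bomb's location.
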(event `self.ReceiveHit`
  (params (MyComp :type "PrimitiveComponent Object Reference") (Other :type "Actor Object Reference") (OtherComp :type "PrimitiveComponent Object Reference") (bSelfMoved :type Boolean) (HitLocation :type "Vector Structure") (HitNormal :type "Vector Structure") (NormalImpulse :type "Vector Structure") (Hit :type "HitResult Structure (by ref)"))
  (bind _outactors (`KismetSystemLibrary.SphereOverlapActors` (`self.K2_GetActorLocation`) 150.0 (`|MakeArray` "ObjectTypeQuery2" :!type "EObjectTypeQuery Enum")))
  (for _array_element _outactors
    (bind _asbp_ufo (cast `/Game/BP-UFO` _array_element))
    (bind _staticmesh (`/Game/BP-UFO.StaticMesh` _asbp_ufo))
    (`PrimitiveComponent.SetSimulatePhysics` _staticmesh true)
    (`TimelineComponent.Stop` (`/Game/BP-UFO.UFO-Animation` _asbp_ufo))
    (`PrimitiveComponent.AddRadialImpulse` _staticmesh (`self.K2_GetActorLocation`) 200.0 1200.0 "RIF_Constant" false)))

(fn `UserConstructionScript`)