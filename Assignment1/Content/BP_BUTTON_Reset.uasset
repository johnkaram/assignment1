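; BP_BUTTON_Reset is a button Blueprint that clears spawned UFOs and bombs from the level when pressed.
; It extends a parent button's ButtonPressed event, then destroys all BPUFO and BP_BOMB actors found by class.
; It also clears and invalidates the timer on the first BP_BUTTON_SpawnBOMBS found, with no check that one exists.
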(event `self.button_pressed`
  (`parent.button_pressed`)
  ;[0 0.4149 1] Destroy UFOs
  (bind _outactors (`GameplayStatics.GetAllActorsOfClass` "/Game/BP-UFO.BP-UFO_C"))
  (`self.K2_DestroyActor` _outactors)
  ;[0.08413 0 1] Destroy BOMBS
  (bind _outactors_2 (`GameplayStatics.GetAllActorsOfClass` "/Game/BP_BOMB.BP_BOMB_C"))
  (`self.K2_DestroyActor` _outactors_2)
  ;[0.7813 0 1] Clear BOMB / Spawn Timer
  (bind _outactors_3 (`GameplayStatics.GetAllActorsOfClass` "/Game/BP_BUTTON_SpawnBOMBS.BP_BUTTON_SpawnBOMBS_C"))
  (`KismetSystemLibrary.K2_ClearAndInvalidateTimerHandle` (`/Game/BP_BUTTON_SpawnBOMBS.timer` (`|GetArrayItem` _outactors_3))))

(fn `UserConstructionScript`
  (`parent.UserConstructionScript`))