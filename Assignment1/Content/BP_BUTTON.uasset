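; BP_BUTTON is an overlap-triggered button that reacts to Pawns entering and leaving it.
; Begin and end overlap call ButtonPressed and ButtonReleased after a Pawn cast.
; The button_pressed event creates a dynamic material instance on Cylinder1 and turns its Emissive parameter green.
; The Button_Released event sets that stored material's Emissive parameter to red.
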(event `self.ReceiveActorBeginOverlap`
  (params (OtherActor :type "Actor Object Reference"))
  (cast `Pawn` OtherActor)
  (`self.button_pressed`))

(event `self.ReceiveActorEndOverlap`
  (params (OtherActor :type "Actor Object Reference"))
  (cast `Pawn` OtherActor)
  (`self.Button_Released`))

(event `button_pressed`
  (bind _returnvalue (`PrimitiveComponent.CreateDynamicMaterialInstance` (`self.Cylinder1`) 0 "/Game/jmaterial_1.jmaterial_1" "None"))
  (bind _output_get (set `self.ButtonMaterial` _returnvalue))
  (`MaterialInstanceDynamic.SetVectorParameterValue` _output_get "Emissive" (struct :`R` 0.048111 :`G` 1.0 :`A` 1.0)))

(event `Button_Released`
  (`MaterialInstanceDynamic.SetVectorParameterValue` (`self.ButtonMaterial`) "Emissive" (struct :`R` 1.0 :`B` 0.049885 :`A` 1.0)))

(fn `UserConstructionScript`)